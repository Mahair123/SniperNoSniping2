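; Sniper scope camera actor that takes over the player's view at BeginPlay and follows the character along a spline path.
; It caches the level's SniperCameraPath_BP and player character at start.
; Each tick it eases the camera toward the spline point closest to the character, queried in local space but applied as world location.
; Only location updates; older rotation and path-following nodes are left disconnected.
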(event Collision|EventActorBeginOverlap
  (params (OtherActor :type Actor%20Object%20Reference)))

(event EventTick
  (params (DeltaSeconds :type Float%20%28single-precision%29))
  (bind _asbp_third_person_character (Utilities|Casting|CastToBP_ThirdPersonCharacter (Variables|Default|GetPlayerCharacterRef)))
  (Transformation|SetWorldLocation (Variables|Default|GetCamera) (Math|Interpolation|VInterpTo (Transformation|GetWorldLocation (Variables|Default|GetCamera)) (Spline|FindLocationClosesttoWorldLocation (Variables|/Game/Camera/SniperCameraPath_BP.SniperCameraPath_BP_C|GetCameraSpline (Variables|Default|GetNickSpline)) (Transformation|GetActorLocation _asbp_third_person_character) "Local") (Utilities|Time|GetWorldDeltaSeconds) 2.0) false false))

(event EventBeginPlay
  (bind _returnvalue (Actor|GetActorOfClass "/Game/Camera/SniperCameraPath_BP.SniperCameraPath_BP_C"))
  (Variables|Default|SetNickSpline _returnvalue)
  (Variables|Default|SetPlayerCharacterRef (Game|GetPlayerCharacter 0))
  (Game|Player|SetViewTargetwithBlend (Game|GetPlayerController (Variables|/Script/Engine.Pawn|GetPlayerState (Game|GetPlayerCharacter 0))) self 0.0 "VTBlend_Linear" 0.0 false))

(fn ConstructionScript)